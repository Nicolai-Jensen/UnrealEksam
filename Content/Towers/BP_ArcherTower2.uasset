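; Archer tower Blueprint that fires arrow projectiles and toggles its range indicator when its mesh is clicked.
; On BeginPlay it enables click events on the player controller and registers itself as the Tower on its AIC_StandardTower AI controller.
; HandleShooting spawns an archer projectile at the arrow spawn point, calls its SpawnBullet, then applies AttackSpeed as the mesh's global animation rate.
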(event OnClicked(Mesh)
  (params (TouchedComponent :type Primitive%20Component%20Object%20Reference) (ButtonPressed :type Key%20Structure :default "None"))
  (bind _towerrange (Variables|Default|GetTowerRange))
  (if (Variables|Default|GetRangeVisable)
    (Development|SetHiddeninGame _towerrange false false)
    (Variables|Default|SetRangeVisable false)
    (else
      (Development|SetHiddeninGame _towerrange true false)
      (Variables|Default|SetRangeVisable true))))

(event EventBeginPlay
  (bind _self self)
  (Variables|/Script/Engine.PlayerController|SetbEnableClickEvents (Game|GetPlayerController 0) true)
  (bind _asaic_standard_tower (Utilities|Casting|CastToAIC_StandardTower (AI|GetAIController _self)))
  (Variables|/Game/Towers/AIC_StandardTower.AIC_StandardTower_C|SetTower _asaic_standard_tower _self))

(fn ConstructionScript)

(fn HandleShooting
  (bind _returnvalue (Game|SpawnActorfromClass "/Game/TopDown/Blueprints/BP_ArcherProjectile.BP_ArcherProjectile_C" (Transformation|GetWorldTransform (Variables|Default|GetArrowSpawnPoint)) "Undefined" "MultiplyWithRoot" 0 0))
  (Default|SpawnBullet _returnvalue "NewEnumerator0")
  ;[1 1 1] ATTACK SPEED SETTER
  (Variables|/Script/Engine.SkeletalMeshComponent|SetGlobalAnimRateScale (Variables|Character|GetMesh) (Variables|Default|GetAttackSpeed)))