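; Lake variant of a big hex terrain tile that animates its surface height to suggest waves.
; BeginPlay starts a timeline that sets the Tile's relative Z directly to the wave height, keeping X and Y.
; Tick repeatedly calls Reverse on that timeline through a random delay of a few seconds, with nothing playing it forward again.
; An outdated, unconnected wave routine that stepped the height in a loop remains in the graph.
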(event EventBeginPlay
  (bind _tile (Variables|Default|GetTile))
  (bind _returnvalue (Transformation|GetRelativeTransform _tile))
  (bind _waveheight (Timeline|Timeline PlayFromStart)
    (:Update
      (Transformation|SetRelativeLocation (Variables|Default|GetTile) (Math|Vector|MakeVector (.x (.location _returnvalue)) (.y (.location _returnvalue)) _waveheight) false false))))

(event EventTick
  (params (DeltaSeconds :type Float%20%28single-precision%29))
  (bind _tile (Variables|Default|GetTile))
  (bind _returnvalue (Transformation|GetRelativeTransform _tile))
  (Utilities|FlowControl|Delay (Math|Random|RandomFloatinRange 0.0 5.0))
  (bind _waveheight (Timeline|Timeline Reverse)
    (:Update
      (Transformation|SetRelativeLocation (Variables|Default|GetTile) (Math|Vector|MakeVector (.x (.location _returnvalue)) (.y (.location _returnvalue)) _waveheight) false false))))

(fn ConstructionScript)